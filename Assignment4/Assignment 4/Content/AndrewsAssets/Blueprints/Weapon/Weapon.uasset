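; Weapon is a pickup actor that hands itself to the player as the current weapon.
; When a MyPlayer overlaps PickupZone, it disables the zone's collision and copies WeaponName to the player's CurrentWeapon.
; It then sets its own class on the player's WeaponCuck child actor component, activates that component and destroys itself, so the same class serves as both pickup and held weapon.
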(event `self.PickupZone.OnComponentBeginOverlap`
  (params (OverlappedComponent :type "PrimitiveComponent Object Reference") (OtherActor :type "Actor Object Reference") (OtherComp :type "PrimitiveComponent Object Reference") (OtherBodyIndex :type Integer) (bFromSweep :type Boolean) (SweepResult :type "HitResult Structure (by ref)"))
  (bind _asmy_player (cast `/Game/AndrewsAssets/Blueprints/MyPlayer` OtherActor)
    (:`then`
      (`PrimitiveComponent.SetCollisionEnabled` (`self.PickupZone`) "NoCollision")
      (set `/Game/AndrewsAssets/Blueprints/MyPlayer.currentWeapon` (`self.weaponName`) _asmy_player)
      (bind _weaponcuck (`/Game/AndrewsAssets/Blueprints/MyPlayer.WeaponCuck` _asmy_player))
      (`ChildActorComponent.SetChildActorClass` _weaponcuck (`GameplayStatics.GetObjectClass` self))
      (`ActorComponent.SetActive` _weaponcuck true false)
      (`self.K2_DestroyActor`))
    (:`CastFailed`
      (`KismetSystemLibrary.PrintString` "Cast \"MyPlayer\" Failed in \"Weapon\":" false true (struct :`R` 1.0 :`B` 0.014578 :`A` 1.0)))))

(fn `UserConstructionScript`)