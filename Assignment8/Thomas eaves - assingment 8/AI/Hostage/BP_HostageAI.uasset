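; Hostage AI Blueprint that maintains the Dead, Injured, Safe and Dormant states of a hostage.
; Each Tick, death triggers a one-time player score penalty, kill count increment and delayed destroy.
; Low health marks it injured and unsafe until health regenerates; otherwise Safe follows a distance scan of all BP_GruntAI actors.
; The player entering its box trigger clears Dormant.
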(event `self.ReceiveBeginPlay`
  (bind _asfirst_person_character (cast `/Game/FirstPersonBPIronbelly/Blueprints/FirstPersonCharacter` (`GameplayStatics.GetPlayerCharacter` 0)))
  (set `self.PlayerCharacterRef` _asfirst_person_character))

(event `self.ReceiveTick`
  (params (DeltaSeconds :type "Float (single-precision)"))
  (bind _playercharacterref (`self.PlayerCharacterRef`))
  (if (`self.IsDead`)
    ;[1 1 1] If dead, take away from players score and add to hostage killed counter, then after delay, destroy self
    (`/Engine/EditorBlueprintResources/StandardMacros.DoOnce` false
      (:`Completed`
        (set `/Game/FirstPersonBPIronbelly/Blueprints/FirstPersonCharacter.Score` (- (`/Game/FirstPersonBPIronbelly/Blueprints/FirstPersonCharacter.Score` _playercharacterref) 25) _playercharacterref)
        (set `/Game/FirstPersonBPIronbelly/Blueprints/FirstPersonCharacter.Hostages Killed` (+ (`/Game/FirstPersonBPIronbelly/Blueprints/FirstPersonCharacter.Hostages Killed` _playercharacterref) 1) _playercharacterref)
        (`KismetSystemLibrary.Delay` 3.0)
        (`self.K2_DestroyActor`)))
    (elif (`self.Injured`)
      ;[1 1 1] If injured, regenerate health, when health is full, set injured to false
      (`/Engine/EditorBlueprintResources/StandardMacros.CompareFloat` (`self.Health`) 100.0
        (:`>`
          (set `self.Injured` false :!label _label))
        (:`==`
          (goto _label))
        (:`<`
          (set `self.Health` (+ (* DeltaSeconds (/ 100.0 10.0)) (`self.Health`)))))
      (else
        ;[1 1 1] If health is low, set injured to ture and set safe to false
        (`/Engine/EditorBlueprintResources/StandardMacros.CompareFloat` (`self.Health`) 20.0
          (:`>`
            ;[1 1 1] Check to see if any Grunts are in range, if so, then set safe to false.
            (bind _outactors (`GameplayStatics.GetAllActorsOfClass` "/Game/AI/Grunt/BP_GruntAI.BP_GruntAI_C"))
            (for _array_element _outactors
              (if (< (`KismetMathLibrary.VSize` (- (`self.K2_GetActorLocation` self) (`self.K2_GetActorLocation` _array_element))) 3000.0)
                (bind _output_get (set `self.HostileInRange` true))))
            (if _output_get
              (set `self.Safe` false)
              (else
                (set `self.Safe` true)))
            (set `self.HostileInRange` false))
          (:`<`
            (set `self.Injured` true)
            (set `self.Safe` false)))))))

(event `self.Box.OnComponentBeginOverlap`
  (params (OverlappedComponent :type "PrimitiveComponent Object Reference") (OtherActor :type "Actor Object Reference") (OtherComp :type "PrimitiveComponent Object Reference") (OtherBodyIndex :type Integer) (bFromSweep :type Boolean) (SweepResult :type "HitResult Structure (by ref)"))
  ;[1 1 1] Check to see if player is in range, if they are, then set dormant to false
  (if (== OtherActor (`GameplayStatics.GetPlayerCharacter` 0))
    (set `self.Dormant` false)))

(fn `UserConstructionScript`)