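; BP_Boss_AI_CON is the boss AI controller, which runs the BT_BossAI behavior tree on BeginPlay.
; When a perception update includes the player, it writes visibility, last stimulus location and target actor to the blackboard from the first sensed stimulus.
; Each such update also spawns a short-lived TargetPoint at the player's current transform, stored as the MemoryMarker key, whether or not sensing succeeded.
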(event `self.ReceiveBeginPlay`
  (`self.RunBehaviorTree` "/Game/AI/Boss/BT_BossAI.BT_BossAI"))

(event `self.AIPerception.OnPerceptionUpdated`
  (params (UpdatedActors :type "Array of Actor Object Reference"))
  (for _array_element UpdatedActors
    (if (== _array_element (`GameplayStatics.GetPlayerCharacter` 0))
      (bind _output_get (set `self.NewEnemy` _array_element))
      (bind _info (`AIPerceptionComponent.GetActorsPerception` (`self.AIPerception`) _output_get))
      (bind (_age _expirationage _strength _stimuluslocation _receiverlocation _tag _bsuccessfullysensed) (break `AIStimulus` (`KismetArrayLibrary.Array_Get` (`.LastSensedStimuli` (break `ActorPerceptionBlueprintInfo` _info)))))
      (`BlackboardComponent.SetValueAsBool` (`AIBlueprintHelperLibrary.GetBlackboard` null) "EnemyVisible" _bsuccessfullysensed)
      (`BlackboardComponent.SetValueAsVector` (`AIBlueprintHelperLibrary.GetBlackboard` null) "MemoryLocation" _stimuluslocation)
      (`BlackboardComponent.SetValueAsObject` (`AIBlueprintHelperLibrary.GetBlackboard` null) "TargetActor" (`self.NewEnemy`))
      (bind _returnvalue (`|SpawnActorFromClass` "/Script/Engine.TargetPoint" (`self.GetTransform` (`GameplayStatics.GetPlayerCharacter` 0)) "Undefined" "OverrideRootScale"))
      (`self.SetLifeSpan` _returnvalue 3.0)
      (`BlackboardComponent.SetValueAsObject` (`AIBlueprintHelperLibrary.GetBlackboard` null) "MemoryMarker" _returnvalue))))

(fn `UserConstructionScript`)