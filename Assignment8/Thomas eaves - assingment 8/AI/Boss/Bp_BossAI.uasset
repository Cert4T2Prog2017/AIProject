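; Boss enemy Blueprint that tracks the boss's health, injury, axe swing and death states on Tick.
; Falling below a health threshold sets Injured and raises Armour, then health regenerates gradually to maximum, where Injured clears and Armour drops.
; On death, a DoOnce awards score and a kill to the cached FirstPersonCharacter, then destroys the boss after a delay.
; The SwingingAxe flag clears itself after a short delay.
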(event `self.ReceiveBeginPlay`
  (bind _asfirst_person_character (cast `/Game/FirstPersonBPIronbelly/Blueprints/FirstPersonCharacter` (`GameplayStatics.GetPlayerCharacter` 0)))
  (set `self.PlayerCHaracterRef` _asfirst_person_character))

(event `self.ReceiveTick`
  (params (DeltaSeconds :type "Float (single-precision)"))
  (bind _playercharacterref (`self.PlayerCHaracterRef`))
  (if (`self.SwingingAxe`)
    (`KismetSystemLibrary.Delay` 1.3)
    (set `self.SwingingAxe` false))
  (if (`self.IsDead`)
    ;[1 1 1] If dead, add to players score and destroy self after a short delay
    (`/Engine/EditorBlueprintResources/StandardMacros.DoOnce` false
      (:`Completed`
        (set `/Game/FirstPersonBPIronbelly/Blueprints/FirstPersonCharacter.Score` (+ (`/Game/FirstPersonBPIronbelly/Blueprints/FirstPersonCharacter.Score` _playercharacterref) 100) _playercharacterref)
        (set `/Game/FirstPersonBPIronbelly/Blueprints/FirstPersonCharacter.EnemysKilled` (+ (`/Game/FirstPersonBPIronbelly/Blueprints/FirstPersonCharacter.EnemysKilled` _playercharacterref) 1) _playercharacterref)
        (`KismetSystemLibrary.Delay` 3.0)
        (`self.K2_DestroyActor`)))
    (elif (`self.Injured`)
      ;[1 1 1] If injured, regenerate health
      (`/Engine/EditorBlueprintResources/StandardMacros.CompareFloat` (`self.Health`) (`self.MaxHealth`)
        (:`>`
          (set `self.Injured` false :!label _label)
          (set `self.Armour` 10.0))
        (:`==`
          (goto _label))
        (:`<`
          (set `self.Health` (+ (`self.Health`) (* DeltaSeconds (/ (`self.MaxHealth`) 20.0))))))
      (else
        ;[1 1 1] Set injured is health is low
        (`/Engine/EditorBlueprintResources/StandardMacros.CompareFloat` (`self.Health`) 75.0
          (:`<`
            (set `self.Injured` true)
            (set `self.Armour` 15.0)))))))

(fn `UserConstructionScript`)