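; BP_GruntAI is a rifle-carrying grunt AI character that manages its own injury and death state.
; Construction attaches the SKScar to the mesh's rifle socket and picks a random skeletal mesh.
; Tick flags low health as Injured, then regenerates health until full before clearing the flag.
; When IsDead is set, it credits the player's score and kill count once, then destroys itself after a delay.
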(event `self.ReceiveBeginPlay`
  (bind _asfirst_person_character (cast `/Game/FirstPersonBPIronbelly/Blueprints/FirstPersonCharacter` (`GameplayStatics.GetPlayerCharacter` 0)))
  (set `self.PlayerCharacterRef` _asfirst_person_character))

(event `self.ReceiveTick`
  (params (DeltaSeconds :type "Float (single-precision)"))
  (bind _playercharacterref (`self.PlayerCharacterRef`))
  (if (`self.IsDead`)
    ;[1 1 1] If dead, add to players score, then after delay, destroy actor
    (`/Engine/EditorBlueprintResources/StandardMacros.DoOnce` false
      (:`Completed`
        (set `/Game/FirstPersonBPIronbelly/Blueprints/FirstPersonCharacter.Score` (+ (`/Game/FirstPersonBPIronbelly/Blueprints/FirstPersonCharacter.Score` _playercharacterref) 10) _playercharacterref)
        (set `/Game/FirstPersonBPIronbelly/Blueprints/FirstPersonCharacter.EnemysKilled` (+ (`/Game/FirstPersonBPIronbelly/Blueprints/FirstPersonCharacter.EnemysKilled` _playercharacterref) 1) _playercharacterref)
        (`KismetSystemLibrary.Delay` 3.0)
        (`self.K2_DestroyActor`)))
    (elif (`self.Injured`)
      ;[1 1 1] If injured, Regenerate Health, When health is full, set injured to false
      (`/Engine/EditorBlueprintResources/StandardMacros.CompareFloat` (`self.Health`) 100.0
        (:`>`
          (set `self.Injured` false :!label _label))
        (:`==`
          (goto _label))
        (:`<`
          (set `self.Health` (+ (* DeltaSeconds (/ (`self.MaxHealth`) 10.0)) (`self.Health`)))))
      (else
        ;[1 1 1] If health is low, Set injured to true
        (`/Engine/EditorBlueprintResources/StandardMacros.CompareFloat` (`self.Health`) 20.0
          (:`<`
            (set `self.Injured` true)))))))

(fn `UserConstructionScript`
  (bind _meshs (`self.meshs`))
  (`SceneComponent.K2_AttachToComponent` (`self.SKScar`) (`self.Mesh`) "RifleSocket" "KeepRelative" "KeepRelative" "KeepRelative" true)
  (`SkinnedMeshComponent.SetSkinnedAssetAndUpdate` (`self.Mesh`) (`KismetArrayLibrary.Array_Get` _meshs (`KismetMathLibrary.RandomIntegerInRange` 0 (- (`KismetArrayLibrary.Array_Length` _meshs) 1))) true))