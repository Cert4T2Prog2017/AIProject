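; BP_BaseCharacter is a character base Blueprint that handles taking damage and dying.
; A HealthDamageInterface event subtracts Damage minus Armour from Health, unclamped, so damage below Armour raises Health.
; When Health drops below zero it sets IsDead.
; Only instances whose class is exactly BP_GruntAI then switch their mesh to physics simulation after a short delay.
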(event `self.ReceiveTick`
  (params (DeltaSeconds :type "Float (single-precision)")))

(event `/Game/AI/BP_HealthInterface.HealthDamageInterface`
  (params (Damage :type "Float (single-precision)"))
  (set `self.Health` (- (`self.Health`) (- Damage (`self.Armour`))))
  (if (> 0.0 (`self.Health`))
    (set `self.IsDead` true)
    (if (== (`GameplayStatics.GetObjectClass` self) "/Game/AI/Grunt/BP_GruntAI.BP_GruntAI_C")
      (`KismetSystemLibrary.Delay` 3.5)
      (`PrimitiveComponent.SetSimulatePhysics` (`self.Mesh`) true))))

(fn `UserConstructionScript`)